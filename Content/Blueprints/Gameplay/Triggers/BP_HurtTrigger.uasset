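; Trigger Blueprint that damages entities active inside it, skipping classes listed in IgnoreTypes.
; On each TriggerTick it loops over ActiveEntities and calls TakeDamage on the HealthComponent of an eligible entity.
; A single CanHurt flag, reset after a Delay, throttles damage across the whole trigger, so one hit blocks the other entities until the cooldown ends.
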(event `self.TriggerTick`
  (params (Delta :type "Float (double-precision)"))
  (for _array_element (`self.ActiveEntities`)
    (if (`KismetArrayLibrary.Array_Contains` (`self.IgnoreTypes`) (`GameplayStatics.GetObjectClass` _array_element))
      _
      (elif (`self.CanHurt`)
        (`HealthComponent.TakeDamage` (`self.GetComponentByClass` _array_element "/Script/Bloodcurdle.HealthComponent") (`self.Damage`))
        (set `self.CanHurt` false)
        (`KismetSystemLibrary.Delay` (`self.Delay`))
        (set `self.CanHurt` true)))))

(fn `UserConstructionScript`
  (`parent.UserConstructionScript`))