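; BP_Teleport_Trigger is a trigger that teleports actors entering it to a set destination.
; On trigger enter, it checks whether the actor's exact class is in ValidTypes, so subclasses of listed types do not match by inheritance.
; Matching actors move in teleport mode to Destination, raised by a fixed vertical offset, and rotate to FaceDir.
; The construction script only calls its parent.
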(event `self.OnTriggerEnter`
  (params (EnteringActor :type "Actor Object Reference"))
  (if (`KismetArrayLibrary.Array_Contains` (`self.ValidTypes`) (`GameplayStatics.GetObjectClass` EnteringActor))
    (`self.K2_SetActorLocationAndRotation` EnteringActor (+ (`self.Destination`) (* (`KismetMathLibrary.Vector_Up`) 64)) (`self.FaceDir`) false true)))

(fn `UserConstructionScript`
  (`parent.UserConstructionScript`))