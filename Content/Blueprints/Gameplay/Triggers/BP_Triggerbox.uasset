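; BP_Triggerbox is a trigger volume Blueprint that tracks which actors are inside it and exposes empty enter, exit and tick events.
; Begin and end overlaps on the Triggerbox component add or remove actors in ActiveEntities, with membership checks so OnTriggerEnter and OnTriggerExit fire only when that list changes.
; Tick forwards delta time to TriggerTick every frame, and all three events act as hooks with no behavior here.
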(event `self.ReceiveTick`
  (params (DeltaSeconds :type "Float (single-precision)"))
  (`self.TriggerTick` DeltaSeconds))

(event `TriggerTick`
  (params (Delta :type "Float (double-precision)")))

(event `OnTriggerEnter`
  (params (EnteringActor :type "Actor Object Reference")))

(event `OnTriggerExit`
  (params (LeavingActor :type "Actor Object Reference")))

(event `self.Triggerbox.OnComponentBeginOverlap`
  (params (OverlappedComponent :type "PrimitiveComponent Object Reference") (OtherActor :type "Actor Object Reference") (OtherComp :type "PrimitiveComponent Object Reference") (OtherBodyIndex :type Integer) (bFromSweep :type Boolean) (SweepResult :type "HitResult Structure (by ref)"))
  (bind _activeentities (`self.ActiveEntities`))
  (if (not (`KismetArrayLibrary.Array_Contains` _activeentities OtherActor))
    (`KismetArrayLibrary.Array_Add` _activeentities OtherActor)
    (`self.OnTriggerEnter` OtherActor)))

(event `self.Triggerbox.OnComponentEndOverlap`
  (params (OverlappedComponent :type "PrimitiveComponent Object Reference") (OtherActor :type "Actor Object Reference") (OtherComp :type "PrimitiveComponent Object Reference") (OtherBodyIndex :type Integer))
  (bind _activeentities (`self.ActiveEntities`))
  (if (`KismetArrayLibrary.Array_Contains` _activeentities OtherActor)
    (`KismetArrayLibrary.Array_RemoveItem` _activeentities OtherActor)
    (`self.OnTriggerExit` OtherActor)))

(fn `UserConstructionScript`)