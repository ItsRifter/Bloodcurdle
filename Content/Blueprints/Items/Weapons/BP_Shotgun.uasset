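; Shotgun weapon Blueprint with a primary shot and a secondary double shot that costs two ammo for twice the pellets.
; Each pellet is a line trace from the owner's camera with random spread, drawn for debugging.
; Secondary hits damage any HealthComponent, while primary only prints hit actor names because its damage logic is disconnected.
; A CanFire flag, reset by timer, enforces the attack delay, slightly longer for secondary fire.
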(event `self.PrimaryFire`
  (bind _returnvalue (`self.GetComponentByClass` (`self.GetOwner`) "/Script/Engine.CameraComponent"))
  (bind _returnvalue_2 (`SceneComponent.K2_GetComponentLocation` _returnvalue))
  (if (>= (`self.CurAmmo`) 1)
    (if (`self.CanFire`)
      (set `self.CanFire` false)
      (`/Engine/EditorBlueprintResources/StandardMacros.DecrementInt` (`self.CurAmmo`)
        (:`  `
          (for _ (range 1 (+ (`self.PelletShots`) 1))
            (bind _outhit (`KismetSystemLibrary.LineTraceSingle` _returnvalue_2 (+ _returnvalue_2 (+ (* (`SceneComponent.GetForwardVector` _returnvalue) 1024.0) (* (`KismetMathLibrary.RandomUnitVector`) 128.0))) "TraceTypeQuery1" false (`|MakeArray` (`self.GetOwner`)) "ForDuration"))
            (`KismetSystemLibrary.PrintString` (`KismetSystemLibrary.GetDisplayName` (`.HitActor` (`GameplayStatics.BreakHitResult` _outhit)))))
          (`KismetSystemLibrary.K2_SetTimer` null "SetCanFire" (`self.AttackDelay`)))))))

(event `self.SecondaryFire`
  (bind _returnvalue (`self.GetComponentByClass` (`self.GetOwner`) "/Script/Engine.CameraComponent"))
  (bind _returnvalue_2 (`SceneComponent.K2_GetComponentLocation` _returnvalue))
  (if (>= (`self.CurAmmo`) 2)
    (if (`self.CanFire`)
      (set `self.CanFire` false)
      (set `self.CurAmmo` (- (`self.CurAmmo`) 2))
      (for _ (range 1 (+ (* (`self.PelletShots`) 2) 1))
        (bind _outhit (`KismetSystemLibrary.LineTraceSingle` _returnvalue_2 (+ _returnvalue_2 (+ (* (`SceneComponent.GetForwardVector` _returnvalue) 1024.0) (* (`KismetMathLibrary.RandomUnitVector`) 128.0))) "TraceTypeQuery1" false (`|MakeArray` (`self.GetOwner`)) "ForDuration"))
        (bind _returnvalue_3 (`self.GetComponentByClass` (`.HitActor` (`GameplayStatics.BreakHitResult` _outhit)) "/Script/Bloodcurdle.HealthComponent"))
        (if (`KismetSystemLibrary.IsValid` _returnvalue_3)
          (`HealthComponent.TakeDamage` _returnvalue_3 (`self.BaseDamage`))))
      (`KismetSystemLibrary.K2_SetTimer` null "SetCanFire" (+ (`self.AttackDelay`) 0.25)))))

(fn `SetCanFire`
  (set `self.CanFire` true))

(fn `UserConstructionScript`)