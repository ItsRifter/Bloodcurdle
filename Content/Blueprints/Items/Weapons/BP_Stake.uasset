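; Stake weapon actor that reacts when its collider overlaps another actor and can deal damage.
; Overlaps with classes outside IgnoreTypes stop collider physics, offset the actor by the collider's world location plus a forward push, and make the other actor its owner.
; If that class is in ValidTypes, it applies fixed damage through a BP_HealthComponent lookup that names no target actor.
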(event `self.Collider.OnComponentBeginOverlap`
  (params (OverlappedComponent :type "PrimitiveComponent Object Reference") (OtherActor :type "Actor Object Reference") (OtherComp :type "PrimitiveComponent Object Reference") (OtherBodyIndex :type Integer) (bFromSweep :type Boolean) (SweepResult :type "HitResult Structure (by ref)"))
  (bind _returnvalue (`GameplayStatics.GetObjectClass` OtherActor))
  (bind _collider (`self.Collider`))
  (if (not (`KismetArrayLibrary.Array_Contains` (`self.IgnoreTypes`) _returnvalue))
    (`PrimitiveComponent.SetSimulatePhysics` _collider false)
    (`self.K2_AddActorWorldOffset` (+ (`SceneComponent.K2_GetComponentLocation` _collider) (* (`SceneComponent.GetForwardVector` _collider) 72)))
    (`self.SetOwner` OtherActor)
    (if (`KismetArrayLibrary.Array_Contains` (`self.ValidTypes`) _returnvalue)
      (`HealthComponent.TakeDamage` (`self.GetComponentByClass` "/Game/Blueprints/BP_HealthComponent.BP_HealthComponent_C") 30.0))))

(fn `UserConstructionScript`)