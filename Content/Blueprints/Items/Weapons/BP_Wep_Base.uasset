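; Base weapon actor that handles player pickup, fire cooldowns and hitscan attack helpers.
; Overlapping its collider adds it to the player's weapons, active if it is the first, and snaps it to the camera at the aim point.
; Primary and secondary fire only gate CanFire with timed delays; separate helpers supply camera aim, sound and line traces.
; Traces damage any actor with a HealthComponent and spawn randomly sized flesh or surface hole decals.
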(event `DoLineTraces`
  (params (Position :type "Vector Structure") (Forward :type "Vector Structure"))
  (bind _asbp_player_character (cast `/Game/Blueprints/Player/BP_PlayerCharacter` (`self.GetOwner`)))
  (bind _outhit (`KismetSystemLibrary.LineTraceSingle` Position Forward "TraceTypeQuery1" false (`|MakeArray` _asbp_player_character :!type "Actor Object Reference")))
  (bind (_bblockinghit _binitialoverlap _time _distance _location _impactpoint _normal _impactnormal _physmat _hitactor) (`GameplayStatics.BreakHitResult` _outhit))
  (bind _result (`self.IsActorNPC` _hitactor))
  (if _result
    (`HealthComponent.TakeDamage` (`self.GetComponentByClass` _hitactor "/Script/Bloodcurdle.HealthComponent") (`self.BaseDamage`))
    (`GameplayStatics.SpawnDecalAtLocation` "/Game/Materials/Mat_Decal_HoleFlesh.Mat_Decal_HoleFlesh" (`KismetMathLibrary.Conv_IntToVector` (`KismetMathLibrary.RandomIntegerInRange` 3 6)) _location (`KismetMathLibrary.Conv_VectorToRotator` _location))
    (else
      (`GameplayStatics.SpawnDecalAtLocation` "/Game/Materials/Mat_Decal_Hole.Mat_Decal_Hole" (`KismetMathLibrary.Conv_IntToVector` (`KismetMathLibrary.RandomIntegerInRange` 3 7)) _location (`KismetMathLibrary.Conv_VectorToRotator` _location) 7.0))))

(event `PlayWeaponSound`
  (params (Sound :type "SoundCue Object Reference") (Pitch :type "Float (double-precision)" :default 1.0))
  (`GameplayStatics.PlaySoundAtLocation` Sound (`self.K2_GetActorLocation` (`self.GetOwner`)) (struct) 1.0 Pitch 0.0 null null null null))

(event `PostFire`
  (params (Time :type "Float (double-precision)" :default 0.1))
  (`KismetSystemLibrary.K2_SetTimerDelegate` (delegate `AllowFire`) Time))

(event `AllowFire`
  (set `self.Can Fire` true))

(event `self.PrimaryFire`
  (set `self.Can Fire` false)
  (`self.PostFire` (`self.AttackDelay`)))

(event `self.SecondaryFire`
  (set `self.Can Fire` false)
  (`self.PostFire` (`self.AltAttackDelay`)))

(event `self.Collider.OnComponentBeginOverlap`
  (params (OverlappedComponent :type "PrimitiveComponent Object Reference") (OtherActor :type "Actor Object Reference") (OtherComp :type "PrimitiveComponent Object Reference") (OtherBodyIndex :type Integer) (bFromSweep :type Boolean) (SweepResult :type "HitResult Structure (by ref)"))
  (bind _asbp_player_character (cast `/Game/Blueprints/Player/BP_PlayerCharacter` OtherActor))
  (`MainPlayerCharacter.AddWeapon` _asbp_player_character self (== (`KismetArrayLibrary.Array_Length` (`MainPlayerCharacter.Weapons` _asbp_player_character)) 0))
  (`self.K2_AttachToComponent` (`MainPlayerCharacter.Camera` _asbp_player_character) "None" "SnapToTarget" "SnapToTarget" "KeepRelative")
  (`self.K2_SetActorRelativeLocation` (`SceneComponent.RelativeLocation` (`/Game/Blueprints/Player/BP_PlayerCharacter.WeaponAimPoint` _asbp_player_character)) false true))

(fn `Get Camera Fire Point`
  (returns (Position :type "Vector Structure") (Forward :type "Vector Structure"))
  (bind _asbp_player_character (cast `/Game/Blueprints/Player/BP_PlayerCharacter` (`self.GetOwner`)))
  (bind _camera (`MainPlayerCharacter.Camera` _asbp_player_character))
  (bind _returnvalue (`SceneComponent.K2_GetComponentLocation` _camera))
  (return _returnvalue (+ _returnvalue (* (`SceneComponent.GetForwardVector` _camera) (`self.AttackRange`)))))

(fn `IsActorNPC`
  (params (Actor :type "Actor Object Reference"))
  (returns (Result :type Boolean))
  (if (`KismetSystemLibrary.IsValid` Actor)
    (if (`KismetSystemLibrary.IsValid` (`self.GetComponentByClass` Actor "/Script/Bloodcurdle.HealthComponent"))
      (return true)
      (else
        (return false)))
    (else
      (return false))))

(fn `IsValidType`
  (params (Actor :type "Actor Class Reference"))
  (returns (Result :type Boolean))
  (return (!= (`KismetArrayLibrary.Array_Find` (`self.ValidTargetTypes`) Actor) -1)))

(fn `UserConstructionScript`)