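; BP_Wep_Shotgun is a double-barrel shotgun weapon with single-shell primary fire and a two-shell secondary blast.
; Each shot spends ammo and loaded shells and runs repeated pellet line traces, with secondary fire doubling pellets and falling back to primary when one shell remains.
; PostFire routes into the parent's cooldown, adding a delayed reload sound, longer wait and up to two-shell refill when empty, while CanFire gates firing.
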(event `self.PrimaryFire`
  (if (>= (`self.CurAmmo`) 1)
    (if (`self.CanFire`)
      (set `self.CanFire` false)
      (set `self.ShotsLeft` (- (`self.ShotsLeft`) 1))
      (`/Engine/EditorBlueprintResources/StandardMacros.DecrementInt` (`self.CurAmmo`)
        (:`  `
          (`self.PlayWeaponSound` "/Game/Sounds/SCue_Shotgun_Fire.SCue_Shotgun_Fire")
          (for _ (range 1 (+ (`self.PelletShots`) 1))
            (`self.DoLineTraces`))
          (`self.PostFire` (`self.AttackDelay`)))))))

(event `self.SecondaryFire`
  (if (>= (`self.CurAmmo`) 2)
    (if (== (`self.ShotsLeft`) 1)
      (`self.PrimaryFire`)
      (elif (`self.CanFire`)
        (set `self.CanFire` false)
        (set `self.ShotsLeft` (- (`self.ShotsLeft`) 2))
        (set `self.CurAmmo` (- (`self.CurAmmo`) 2))
        (`self.PlayWeaponSound` "/Game/Sounds/SCue_Shotgun_Fire.SCue_Shotgun_Fire")
        (for _ (range 1 (+ (* (`self.PelletShots`) 2) 1))
          (`self.DoLineTraces`))
        (`self.PostFire` (+ (`self.AttackDelay`) 0.25))))))

(event `self.PostFire`
  (params (Time :type "Float (double-precision)"))
  (if (<= (`self.ShotsLeft`) 0)
    (`KismetSystemLibrary.Delay` 0.4)
    (`self.PlayWeaponSound` "/Game/Sounds/SCue_Shotgun_Reload.SCue_Shotgun_Reload")
    (`parent.PostFire` (+ (`self.AttackDelay`) 0.95))
    (set `self.ShotsLeft` (`KismetMathLibrary.Min` (`self.CurAmmo`) 2))
    (else
      (`parent.PostFire` Time))))

(event `self.AllowFire`
  (set `self.CanFire` true))

(fn `UserConstructionScript`)