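; Stakebow weapon Blueprint that fires physical stake projectiles and offers a toggleable zoom.
; Primary fire, gated by CanWeaponShoot, spawns a BP_Stake just ahead of and above the owner, launches it with a velocity-change impulse, spends ammo and calls the parent.
; Secondary fire toggles a narrowed player camera FOV and hides the weapon mesh while zoomed.
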(event `self.PrimaryFire`
  (bind _returnvalue (`self.GetOwner`))
  (bind _returnvalue_2 (+ (+ (* (`KismetMathLibrary.Vector_Up`) 26.0) (`self.K2_GetActorLocation` _returnvalue)) (* (`self.GetActorForwardVector` _returnvalue) 16.0)))
  ;[1 1 1] Launches stake
  (`/Game/Blueprints/Items/Weapons/BPMac_Weapons.CanWeaponShoot`
    (:`True`
      (bind _returnvalue_3 (`|SpawnActorFromClass` "/Game/Blueprints/Items/Weapons/BP_Stake.BP_Stake_C" (`KismetMathLibrary.MakeTransform` _returnvalue_2 (`SceneComponent.K2_GetComponentRotation` (`self.Weapon`))) "Undefined" "MultiplyWithRoot" null null))
      (`PrimitiveComponent.AddVelocityChangeImpulseAtLocation` (`/Game/Blueprints/Items/Weapons/BP_Stake.Collider` _returnvalue_3) (* (`self.GetActorForwardVector`) (* 1024.0 5.0)) _returnvalue_2 "None")
      (`/Engine/EditorBlueprintResources/StandardMacros.DecrementInt` (`self.CurAmmo`)
        (:`  `
          (`parent.PrimaryFire`))))))

(event `self.SecondaryFire`
  (bind _weapon (`self.Weapon`))
  ;[1 1 1] Zoom toggle
  (bind _asbp_player_character (cast `/Game/Blueprints/Player/BP_PlayerCharacter` (`self.GetOwner`)))
  (if (`self.IsZoomed`)
    (set `self.IsZoomed` false)
    (bind _camera (`MainPlayerCharacter.Camera` _asbp_player_character))
    (`CameraComponent.SetFieldOfView` _camera 90.0)
    (`SceneComponent.SetVisibility` _weapon true false)
    (else
      (set `self.IsZoomed` true)
      (`CameraComponent.SetFieldOfView` _camera 35.0)
      (`SceneComponent.SetVisibility` _weapon false false))))

(fn `UserConstructionScript`
  (`parent.UserConstructionScript`))