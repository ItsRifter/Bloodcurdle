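; BP_Wep_Sword is a melee weapon Blueprint that deals damage to whatever the wielder is looking at within attack range.
; Primary fire runs a single Visibility line trace from the owner's camera along its forward vector, ignoring the owner and drawing debug lines.
; A valid hit actor takes base damage through its HealthComponent, fetched without a check that the component exists.
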(event `self.PrimaryFire`
  (`self.DoLineTraces`))

(event `self.DoLineTraces`
  (bind _returnvalue (`self.GetComponentByClass` (`self.GetOwner`) "/Script/Engine.CameraComponent"))
  (bind _returnvalue_2 (`SceneComponent.K2_GetComponentLocation` _returnvalue))
  (bind _outhit (`KismetSystemLibrary.LineTraceSingle` _returnvalue_2 (+ _returnvalue_2 (* (`SceneComponent.GetForwardVector` _returnvalue) (`self.AttackRange`))) "TraceTypeQuery1" false (`|MakeArray` (`self.GetOwner`)) "ForDuration"))
  (bind (_bblockinghit _binitialoverlap _time _distance _location _impactpoint _normal _impactnormal _physmat _hitactor) (`GameplayStatics.BreakHitResult` _outhit))
  (bind _result (`self.IsValidTypeRef` _hitactor))
  (if _result
    (`HealthComponent.TakeDamage` (`self.GetComponentByClass` _hitactor "/Script/Bloodcurdle.HealthComponent") (`self.BaseDamage`))))

(fn `UserConstructionScript`
  (`parent.UserConstructionScript`))