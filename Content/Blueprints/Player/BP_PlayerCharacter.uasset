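; Player character Blueprint that manages the HUD, weapon fire and death handling.
; On BeginPlay it creates and sets up the HUD widget, and its fire events forward to the active weapon while the player is alive.
; When Health reports death, it signals game over to BP_BCGame, then drops and rotates the camera.
; Jump input restarts the game through the game mode when gameplay status matches a specific state.
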(event `self.ReceiveBeginPlay`
  ;[1 1 1] Setup player
  (set `self.IsAlive` true)
  (bind _returnvalue (`|CreateWidget` "/Game/Blueprints/UI/UI_PlayerHud.UI_PlayerHud_C" (`GameplayStatics.GetPlayerController` 0)))
  (bind _output_get (set `self.HUD` _returnvalue))
  (`/Game/Blueprints/UI/UI_PlayerHud.Setup` _output_get self)
  (`UserWidget.AddToViewport` _output_get 0))

(event `self.DoPrimaryFire`
  (bind _activeweapon (`self.ActiveWeapon`))
  ;[1 1 1] Weapon action events
  ;;[0.2083 1 0.2432] On Primary fire - Left mouse button pressed
  (if (`self.IsAlive`)
    (`/Engine/EditorBlueprintResources/StandardMacros.IsValid` _activeweapon
      (:`Is Valid`
        (`WeaponBase.PrimaryFire` _activeweapon)))))

(event `self.DoSecondaryFire`
  (bind _activeweapon (`self.ActiveWeapon`))
  ;[1 1 1] Weapon action events
  ;;[0 1 0.6697] On Secondary fire - Right mouse button pressed
  (if (`self.IsAlive`)
    (`/Engine/EditorBlueprintResources/StandardMacros.IsValid` _activeweapon
      (:`Is Valid`
        (`WeaponBase.SecondaryFire` _activeweapon)))))

(event `self.Health.OnOwnerDied`
  ;[1 1 1] Player died
  (bind _asbp_bcgame (cast `/Game/Blueprints/Gameplay/BP_BCGame` (`GameplayStatics.GetGameMode`)))
  (`/Game/Blueprints/Gameplay/BP_BCGame.EventGameOver` _asbp_bcgame)
  (`self.DoDeath`))

(event `DoDeath`
  ;[1 1 1] Perform death functions
  (set `self.IsAlive` false)
  (`SceneComponent.K2_AddLocalOffset` (`self.Camera`) (0.0 0.0 -90.0) false false)
  (`SceneComponent.K2_AddLocalRotation` (`self.Camera`) (struct :`Roll` 30.0) false false))

(event `EnhancedInput|/Game/Blueprints/Input/IA_Jump`
  (params (ActionValue :type Boolean) (ElapsedSeconds :type "Float (double-precision)") (TriggeredSeconds :type "Float (double-precision)") (InputAction :type "InputAction Object Reference" :default "/Game/Blueprints/Input/IA_Jump.IA_Jump"))
  (:`Triggered`
    (bind _asbp_bcgame (cast `/Game/Blueprints/Gameplay/BP_BCGame` (`GameplayStatics.GetGameMode`)))
    (if (`|EnumEquality` (`/Game/Blueprints/Gameplay/BP_BCGame.GameplayStatus` _asbp_bcgame) "NewEnumerator2")
      (if ActionValue
        (`/Game/Blueprints/Gameplay/BP_BCGame.RestartGame` _asbp_bcgame)))))

(fn `UserConstructionScript`)